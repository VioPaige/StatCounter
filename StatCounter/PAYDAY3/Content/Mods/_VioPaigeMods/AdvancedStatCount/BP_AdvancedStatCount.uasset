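; Mod actor that keeps persistent player stats across heists: kills by enemy type plus revives, minigames, explosions, objectives and threat level.
; BeginPlay loads or recreates the save, retries until the local player exists, then binds to the game event broker and level actors, and polls threat level.
; Handlers increment counters (kills via a class-to-int map), call SaveKills and refresh the widget.
; FBI van counts are never saved, and cooking-station changes are only logged.
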(event `self.ReceiveBeginPlay`
  (bind _lastthreatlevel (`self.LastThreatLevel`))
  (`|ExecutionSequence`
    (:`then_0`
      (bind _returnvalue (`GameplayStatics.DoesSaveGameExist` "AdvancedKillCountSave"))
      (if _returnvalue
        (`/Game/Mods/ModLoader/Blueprints/Utilities/BPFL_ModLoader.PrintToModLoader` "Found a save, loading..")
        (bind _returnvalue_2 (`GameplayStatics.LoadGameFromSlot` "AdvancedKillCountSave"))
        (bind _asbp_advanced_stat_count_save (cast `/Game/Mods/_VioPaigeMods/AdvancedStatCount/BP_AdvancedStatCountSave` _returnvalue_2))
        (set `self.Save` _asbp_advanced_stat_count_save)
        (`self.LoadKills`)
        (`KismetSystemLibrary.Delay` 0.2)
        (if (not (`self.FirstLoad`))
          (`/Game/Mods/ModLoader/Blueprints/Utilities/BPFL_ModLoader.PrintToModLoader` "Clearing Old AKC Save...")
          (`GameplayStatics.DeleteGameInSlot` "AdvancedKillCountSave")
          (set `self.FirstLoad` true)
          (`/Game/Mods/ModLoader/Blueprints/Utilities/BPFL_ModLoader.PrintToModLoader` "Creating new save" :!label _label)
          (bind _returnvalue_3 (`GameplayStatics.CreateSaveGameObject` "/Game/Mods/_VioPaigeMods/AdvancedStatCount/BP_AdvancedStatCountSave.BP_AdvancedStatCountSave_C"))
          (bind _output_get (set `self.Save` _returnvalue_3))
          (set `/Game/Mods/_VioPaigeMods/AdvancedStatCount/BP_AdvancedStatCountSave.FirstLoadDone` true _output_get)
          (`GameplayStatics.SaveGameToSlot` _output_get "AdvancedKillCountSave")
          (`/Game/Mods/ModLoader/Blueprints/Utilities/BPFL_ModLoader.PrintToModLoader` (`KismetStringLibrary.Concat_StrStr` "Value of total kills: " (`KismetStringLibrary.Conv_IntToString` (`/Game/Mods/_VioPaigeMods/AdvancedStatCount/BP_AdvancedStatCountSave.Total` _output_get)))))
        (else
          (goto _label))))
    (:`then_1`
      ;[0 0 0] Set Player Variable
      (bind _assbzplayer_character (cast `SBZPlayerCharacter` (`SBZPlayerLibrary.GetLocalPlayerPawn`) :!label _label_2)
        (:`then`
          (set `self.LocalPlayer` _assbzplayer_character)
          (bind _returnvalue_4 (`SBZEventLibrary.GetGameEventBroker`))
          (`|ExecutionSequence`
            (:`then_0`
              (add `SBZGameEventBroker.OnTakenDamage` _returnvalue_4 (delegate `OnTakenDamage`)))
            (:`then_1`
              (add `SBZGameEventBroker.OnRevive` _returnvalue_4 (delegate `OnRevive`)))
            (:`then_2`
              (bind _outactors (`GameplayStatics.GetAllActorsOfClass` "/Script/Starbreeze.SBZMiniGameActor"))
              (for _array_element _outactors
                (add `SBZMiniGameActor.OnMiniGameSuccessful` _array_element (delegate `MinigameSuccess`))))
            (:`then_3`
              (bind _outactors_2 (`GameplayStatics.GetAllActorsOfClass` "/Script/Starbreeze.SBZExplosiveLevelProp"))
              (for _array_element_2 _outactors_2
                (add `SBZExplosiveLevelProp.ServerOnExploded` _array_element_2 (delegate `OnPropExplode`))))
            (:`then_4`
              (bind _outactors_3 (`GameplayStatics.GetAllActorsOfClass` "/Script/Starbreeze.SBZMissionState"))
              (for _array_element_3 _outactors_3
                (add `SBZMissionState.OnFBIActivationChanged` _array_element_3 (delegate `OnFBIChanged`))))
            (:`then_5`
              (bind _outactors_4 (`GameplayStatics.GetAllActorsOfClass` "/Script/Starbreeze.SBZObjective"))
              (for _array_element_4 _outactors_4
                (add `SBZObjective.OnCompleted` _array_element_4 (delegate `OnObjectiveComplete`))))
            (:`then_6`
              (bind _outactors_5 (`GameplayStatics.GetAllActorsOfClass` "/Script/Starbreeze.SBZCookingStation" :!label _label_3))
              (for _array_element_5 _outactors_5
                (`/Game/Mods/ModLoader/Blueprints/Utilities/BPFL_ModLoader.PrintToModLoader` "Found Cooking Station")
                (set `self.FoundStation` true)
                (add `SBZCookingStation.OnRequiredIngredientChanged` _array_element_5 (delegate `OnIngredientChanged`)))
              (`/Game/Mods/ModLoader/Blueprints/Utilities/BPFL_ModLoader.PrintToModLoader` "Finished looping through cooking stations")
              (if (not (`self.FoundStation`))
                (`KismetSystemLibrary.Delay` 10.0)
                (goto _label_3)))
            (:`then_7`
              (bind _outactors_6 (`GameplayStatics.GetAllActorsOfClass` "/Game/Gameplay/Modes/BP_HeistGameState.BP_HeistGameState_C"))
              (for _array_element_6 _outactors_6
                (bind _currentthreatlevel (`PD3HeistGameState.CurrentThreatLevel` _array_element_6))
                (if (not (== _currentthreatlevel _lastthreatlevel)) :!label _label_4
                  (set `self.SavedThreatLevel` (+ (- _currentthreatlevel _lastthreatlevel) (`self.SavedThreatLevel`)))
                  (set `self.LastThreatLevel` _currentthreatlevel))
                (`KismetSystemLibrary.Delay` 5.0)
                (goto _label_4)))))
        (:`CastFailed`
          (`KismetSystemLibrary.Delay` 0.2)
          (goto _label_2))))))

(event `OnTakenDamage`
  (params (DamageEventData :type "SBZDamageEvent Structure (by ref)"))
  (bind (_attacker _causer _victim _equippabledata _throwabledata _damage _armordamage _healthdamage _overhealdamage _bcritical _bwasarmorbroken _biskillshot) (break `SBZDamageEvent` DamageEventData))
  (bind _charactertointmap (`self.CharacterToIntMAP`))
  (bind _returnvalue (`GameplayStatics.GetObjectClass` _victim))
  (bind (_value _returnvalue_2) (`BlueprintMapLibrary.Map_Find` _charactertointmap _returnvalue))
  (bind _assbzplayer_character (cast `SBZPlayerCharacter` _attacker))
  (if (and (== _assbzplayer_character (`self.LocalPlayer`)) _biskillshot)
    (if (or (== _returnvalue "/Game/Gameplay/Characters/Cop/CH_SWAT_AR_HEAVY.CH_SWAT_AR_HEAVY_C") (== _returnvalue "/Game/Gameplay/Characters/Cop/CH_SWAT_Shotgun_HEAVY.CH_SWAT_Shotgun_HEAVY_C") (== _returnvalue "/Game/Gameplay/Characters/Cop/CH_SWAT_SMG_HEAVY.CH_SWAT_SMG_HEAVY_C"))
      (`/Engine/EditorBlueprintResources/StandardMacros.IncrementInt` (`self.HeavyKills`)
        (:`  `
          (`/Engine/EditorBlueprintResources/StandardMacros.IncrementInt` (`self.TotalKills`)
            (:`  `
              (`self.SaveKills`)
              (`/Game/Mods/_VioPaigeMods/AdvancedStatCount/StatCountWidget.UpdateUI` (`self.Widget`))))))
      (elif (`BlueprintMapLibrary.Map_Contains` (`self.CharacterToIntMAP`) _returnvalue)
        (bind _keys (`BlueprintMapLibrary.Map_Keys` _charactertointmap))
        (for _array_element _keys
          (if (and _returnvalue_2 (== _array_element _returnvalue))
            (bind _result (`/Engine/EditorBlueprintResources/StandardMacros.IncrementInt` _value)
              (:`  `
                (`BlueprintMapLibrary.Map_Add` _charactertointmap _array_element _result)
                (`/Engine/EditorBlueprintResources/StandardMacros.IncrementInt` (`self.TotalKills`)
                  (:`  `
                    (`self.SaveKills`)
                    (`/Game/Mods/_VioPaigeMods/AdvancedStatCount/StatCountWidget.UpdateUI` (`self.Widget`))))))))
        (else
          (`/Engine/EditorBlueprintResources/StandardMacros.IncrementInt` (`self.OtherKills`)
            (:`  `
              (`/Engine/EditorBlueprintResources/StandardMacros.IncrementInt` (`self.TotalKills`)
                (:`  `
                  (`self.SaveKills`)
                  (`/Game/Mods/_VioPaigeMods/AdvancedStatCount/StatCountWidget.UpdateUI` (`self.Widget`)))))))))))

(event `OnRevive`
  (params (ReviveEventData :type "SBZReviveEvent Structure (by ref)"))
  (bind (_reviver _characterbeingrevived) (break `SBZReviveEvent` ReviveEventData))
  (bind _localplayer (`self.LocalPlayer`))
  (`|ExecutionSequence`
    (:`then_0`
      (if (== _reviver _localplayer)
        (`/Engine/EditorBlueprintResources/StandardMacros.IncrementInt` (`self.Revived`)
          (:`  `
            (`self.SaveKills` :!label _label_5)
            (`/Game/Mods/_VioPaigeMods/AdvancedStatCount/StatCountWidget.UpdateUI` (`self.Widget`))))))
    (:`then_1`
      (if (== _characterbeingrevived _localplayer)
        (`/Engine/EditorBlueprintResources/StandardMacros.IncrementInt` (`self.GotRevived`)
          (:`  `
            (goto _label_5)))))))

(event `MinigameSuccess`
  (`/Engine/EditorBlueprintResources/StandardMacros.IncrementInt` (`self.Minigames`)
    (:`  `
      (`self.SaveKills`)
      (`/Game/Mods/_VioPaigeMods/AdvancedStatCount/StatCountWidget.UpdateUI` (`self.Widget`)))))

(event `OnPropExplode`
  (`/Engine/EditorBlueprintResources/StandardMacros.IncrementInt` (`self.Explosives`)
    (:`  `
      (`self.SaveKills`)
      (`/Game/Mods/_VioPaigeMods/AdvancedStatCount/StatCountWidget.UpdateUI` (`self.Widget`)))))

(event `OnFBIChanged`
  (params (bIsActive :type Boolean))
  (if (not bIsActive)
    (`/Game/Mods/ModLoader/Blueprints/Utilities/BPFL_ModLoader.PrintToModLoader` "FBI is gone")
    (`/Engine/EditorBlueprintResources/StandardMacros.IncrementInt` (`self.FBIVans`)
      (:`  `
        (`self.SaveKills`)
        (`/Game/Mods/_VioPaigeMods/AdvancedStatCount/StatCountWidget.UpdateUI` (`self.Widget`))))))

(event `OnObjectiveComplete`
  (`/Engine/EditorBlueprintResources/StandardMacros.IncrementInt` (`self.Objectives`)
    (:`  `
      (`self.SaveKills`)
      (`/Game/Mods/_VioPaigeMods/AdvancedStatCount/StatCountWidget.UpdateUI` (`self.Widget`)))))

(event `OnIngredientChanged`
  (params (NewIngredientIndex :type Integer))
  (`/Game/Mods/ModLoader/Blueprints/Utilities/BPFL_ModLoader.PrintToModLoader` (`KismetStringLibrary.Concat_StrStr` "New Ingredient index" (`KismetStringLibrary.Conv_IntToString` NewIngredientIndex))))

(fn `LoadKills`
  (bind _save (`self.Save`))
  (bind _charactertointmap (`self.CharacterToIntMAP`))
  (`|ExecutionSequence`
    (:`then_0`
      (set `self.FirstLoad` (`/Game/Mods/_VioPaigeMods/AdvancedStatCount/BP_AdvancedStatCountSave.FirstLoadDone` _save))
      (set `self.TotalKills` (`/Game/Mods/_VioPaigeMods/AdvancedStatCount/BP_AdvancedStatCountSave.Total` _save))
      (set `self.OtherKills` (`/Game/Mods/_VioPaigeMods/AdvancedStatCount/BP_AdvancedStatCountSave.Other` _save))
      (set `self.HeavyKills` (`/Game/Mods/_VioPaigeMods/AdvancedStatCount/BP_AdvancedStatCountSave.HeavySWAT` _save))
      (bind _keys (`BlueprintMapLibrary.Map_Keys` _charactertointmap))
      (for _array_element _keys
        (`self.SwitchOnCharacter` _array_element
          (:`CH_SecurityGuard`
            (`BlueprintMapLibrary.Map_Add` _charactertointmap _array_element (`/Game/Mods/_VioPaigeMods/AdvancedStatCount/BP_AdvancedStatCountSave.Guard` _save)))
          (:`CH_Dozer`
            (`BlueprintMapLibrary.Map_Add` _charactertointmap _array_element (`/Game/Mods/_VioPaigeMods/AdvancedStatCount/BP_AdvancedStatCountSave.Dozer` _save)))
          (:`CH_Cloaker`
            (`BlueprintMapLibrary.Map_Add` _charactertointmap _array_element (`/Game/Mods/_VioPaigeMods/AdvancedStatCount/BP_AdvancedStatCountSave.Cloaker` _save)))
          (:`CH_Grenadier`
            (`BlueprintMapLibrary.Map_Add` _charactertointmap _array_element (`/Game/Mods/_VioPaigeMods/AdvancedStatCount/BP_AdvancedStatCountSave.Grenadier` _save)))
          (:`CH_Taser`
            (`BlueprintMapLibrary.Map_Add` _charactertointmap _array_element (`/Game/Mods/_VioPaigeMods/AdvancedStatCount/BP_AdvancedStatCountSave.Taser` _save)))
          (:`CH_Sniper`
            (`BlueprintMapLibrary.Map_Add` _charactertointmap _array_element (`/Game/Mods/_VioPaigeMods/AdvancedStatCount/BP_AdvancedStatCountSave.Sniper` _save)))
          (:`CH_SWAT_SHIELD`
            (`BlueprintMapLibrary.Map_Add` _charactertointmap _array_element (`/Game/Mods/_VioPaigeMods/AdvancedStatCount/BP_AdvancedStatCountSave.Shield` _save))))))
    (:`then_1`
      (set `self.Explosives` (`/Game/Mods/_VioPaigeMods/AdvancedStatCount/BP_AdvancedStatCountSave.Explosives` _save))
      (set `self.Minigames` (`/Game/Mods/_VioPaigeMods/AdvancedStatCount/BP_AdvancedStatCountSave.Minigames` _save))
      (set `self.Minigames` (`/Game/Mods/_VioPaigeMods/AdvancedStatCount/BP_AdvancedStatCountSave.Minigames` _save))
      (set `self.Revived` (`/Game/Mods/_VioPaigeMods/AdvancedStatCount/BP_AdvancedStatCountSave.Revived` _save))
      (set `self.GotRevived` (`/Game/Mods/_VioPaigeMods/AdvancedStatCount/BP_AdvancedStatCountSave.GotRevived` _save))
      (set `self.Objectives` (`/Game/Mods/_VioPaigeMods/AdvancedStatCount/BP_AdvancedStatCountSave.Objectives` _save))
      (set `self.SavedThreatLevel` (`/Game/Mods/_VioPaigeMods/AdvancedStatCount/BP_AdvancedStatCountSave.ThreatLevel` _save)))))

(fn `SaveKills`
  (bind _save (`self.Save`))
  (bind _charactertointmap (`self.CharacterToIntMAP`))
  (`|ExecutionSequence`
    (:`then_0`
      (set `/Game/Mods/_VioPaigeMods/AdvancedStatCount/BP_AdvancedStatCountSave.Total` (`self.TotalKills`) _save)
      (set `/Game/Mods/_VioPaigeMods/AdvancedStatCount/BP_AdvancedStatCountSave.Other` (`self.OtherKills`) _save)
      (set `/Game/Mods/_VioPaigeMods/AdvancedStatCount/BP_AdvancedStatCountSave.HeavySWAT` (`self.HeavyKills`) _save)
      (bind _keys (`BlueprintMapLibrary.Map_Keys` _charactertointmap))
      (for _array_element _keys
        (`self.SwitchOnCharacter` _array_element
          (:`CH_SecurityGuard`
            (bind _value (`BlueprintMapLibrary.Map_Find` _charactertointmap _array_element))
            (set `/Game/Mods/_VioPaigeMods/AdvancedStatCount/BP_AdvancedStatCountSave.Guard` _value _save))
          (:`CH_Dozer`
            (set `/Game/Mods/_VioPaigeMods/AdvancedStatCount/BP_AdvancedStatCountSave.Dozer` _value _save))
          (:`CH_Cloaker`
            (set `/Game/Mods/_VioPaigeMods/AdvancedStatCount/BP_AdvancedStatCountSave.Cloaker` _value _save))
          (:`CH_Grenadier`
            (set `/Game/Mods/_VioPaigeMods/AdvancedStatCount/BP_AdvancedStatCountSave.Grenadier` _value _save))
          (:`CH_Taser`
            (set `/Game/Mods/_VioPaigeMods/AdvancedStatCount/BP_AdvancedStatCountSave.Taser` _value _save))
          (:`CH_Sniper`
            (set `/Game/Mods/_VioPaigeMods/AdvancedStatCount/BP_AdvancedStatCountSave.Sniper` _value _save))
          (:`CH_SWAT_SHIELD`
            (set `/Game/Mods/_VioPaigeMods/AdvancedStatCount/BP_AdvancedStatCountSave.Shield` _value _save)))
        (`GameplayStatics.SaveGameToSlot` _save "AdvancedKillCountSave")))
    (:`then_1`
      (set `/Game/Mods/_VioPaigeMods/AdvancedStatCount/BP_AdvancedStatCountSave.Explosives` (`self.Explosives`) _save)
      (set `/Game/Mods/_VioPaigeMods/AdvancedStatCount/BP_AdvancedStatCountSave.Minigames` (`self.Minigames`) _save)
      (set `/Game/Mods/_VioPaigeMods/AdvancedStatCount/BP_AdvancedStatCountSave.Minigames` (`self.Minigames`) _save)
      (set `/Game/Mods/_VioPaigeMods/AdvancedStatCount/BP_AdvancedStatCountSave.Revived` (`self.Revived`) _save)
      (set `/Game/Mods/_VioPaigeMods/AdvancedStatCount/BP_AdvancedStatCountSave.GotRevived` (`self.GotRevived`) _save)
      (set `/Game/Mods/_VioPaigeMods/AdvancedStatCount/BP_AdvancedStatCountSave.Objectives` (`self.Objectives`) _save)
      (set `/Game/Mods/_VioPaigeMods/AdvancedStatCount/BP_AdvancedStatCountSave.ThreatLevel` (`self.SavedThreatLevel`) _save))
    (:`then_2`
      (`GameplayStatics.SaveGameToSlot` _save "AdvancedKillCountSave"))))

(fn `UserConstructionScript`
  (`parent.UserConstructionScript`))